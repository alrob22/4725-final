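; Parent Blueprint for an interactable actor that shows a widget while something overlaps its sphere.
; The E key input prints a debug message and applies a small fixed impulse to the Cube, with no check on the overlap state.
; A separate Interact event prints a message and swaps the first material slot on the attach parent actor's static mesh to GreyedOut.
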(event OnComponentBeginOverlap(Sphere)
  (params (OverlappedComponent :type Primitive%20Component%20Object%20Reference) (OtherActor :type Actor%20Object%20Reference) (OtherComp :type Primitive%20Component%20Object%20Reference) (OtherBodyIndex :type Integer) (bFromSweep :type Boolean) (SweepResult :type Hit%20Result%20Structure%20%28by%20ref%29))
  (Rendering|SetVisibility (Variables|Default|GetWidget) true false))

(event OnComponentEndOverlap(Sphere)
  (params (OverlappedComponent :type Primitive%20Component%20Object%20Reference) (OtherActor :type Actor%20Object%20Reference) (OtherComp :type Primitive%20Component%20Object%20Reference) (OtherBodyIndex :type Integer))
  (Rendering|SetVisibility (Variables|Default|GetWidget) false false))

(event Input|EnhancedActionEvents|EnhancedInputActionIA_EKey
  (params (ActionValue :type Boolean) (ElapsedSeconds :type Float%20%28double-precision%29) (TriggeredSeconds :type Float%20%28double-precision%29) (InputAction :type Input%20Action%20Object%20Reference :default "/Game/FirstPerson/Input/Actions/IA_EKey.IA_EKey"))
  (Development|PrintString "Pushed E")
  (Physics|AddImpulse (Variables|Default|GetCube) "5.000000,5.000000,0.000000" "None" false))

(event EventInteract
  (Development|PrintString "interacting" true true "(R=0.000000,G=0.660000,B=1.000000,A=1.000000)" 3.0)
  (Rendering|Material|SetMaterial (Actor|GetComponentbyClass (Actor|GetAttachParentActor) "/Script/Engine.StaticMeshComponent") 0 "/Game/Objects/Ship2_obj/GreyedOut.GreyedOut"))

(fn ConstructionScript)