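; An interactable cube that passes its ColorIndex to the first-person character and animates its own material when used.
; A sphere overlap toggles a prompt widget, and a separate E-key input nudges the cube with an impulse.
; Interact is gated by the Scucced flag, which it clears, then derives a center from the actor under the cursor.
; A timeline feeds that center and a growing radius into the cube's dynamic material.
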(event OnComponentBeginOverlap(Sphere)
  (params (OverlappedComponent :type Primitive%20Component%20Object%20Reference) (OtherActor :type Actor%20Object%20Reference) (OtherComp :type Primitive%20Component%20Object%20Reference) (OtherBodyIndex :type Integer) (bFromSweep :type Boolean) (SweepResult :type Hit%20Result%20Structure%20%28by%20ref%29))
  (Rendering|SetVisibility (Variables|Components|GetWidget) true false))

(event OnComponentEndOverlap(Sphere)
  (params (OverlappedComponent :type Primitive%20Component%20Object%20Reference) (OtherActor :type Actor%20Object%20Reference) (OtherComp :type Primitive%20Component%20Object%20Reference) (OtherBodyIndex :type Integer))
  (Rendering|SetVisibility (Variables|Components|GetWidget) false false))

(event Custom|this%20time
  (params (PlayRate :type Float%20%28single-precision%29) (Center :type Vector%202D%20Structure))
  (bind (_x _y) (Math|Vector2D|BreakVector2D Center))
  (bind _dynamicmaterial (Variables|Default|GetDynamicMaterial))
  (Development|PrintString "MEEEEE")
  (Components|Timeline|SetPlayRate (Variables|Default|GetTL_Drop) PlayRate)
  (bind _newtrack_1 (Timeline|TL_Drop PlayFromStart)
    (:Update
      (Rendering|Material|SetScalarParameterValue _dynamicmaterial "radius" (* _newtrack_1 2.0) :!class /Script/Engine.MaterialInstanceDynamic)
      (Rendering|Material|SetVectorParameterValue _dynamicmaterial "center" (Utilities|Struct|MakeLinearColor _x _y 0.0 1.0) :!class /Script/Engine.MaterialInstanceDynamic))))

(event Input|EnhancedActionEvents|EnhancedInputActionIA_EKey
  (params (ActionValue :type Boolean) (ElapsedSeconds :type Float%20%28double-precision%29) (TriggeredSeconds :type Float%20%28double-precision%29) (InputAction :type Input%20Action%20Object%20Reference :default "/Game/FirstPerson/Input/Actions/IA_EKey.IA_EKey"))
  (Development|PrintString "Pushed E")
  (Physics|AddImpulse (Variables|Components|GetCube) "5.000000,5.000000,0.000000" "None" false))

(event EventBeginPlay
  (bind _cube (Variables|Components|GetCube))
  (bind _returnvalue (Rendering|Material|CreateDynamicMaterialInstance _cube 0 (Variables|Default|GetSoruceColor) "None" :!class /Script/Engine.PrimitiveComponent))
  (bind _output_get (Variables|Default|SetDynamicMaterial _returnvalue))
  (Rendering|Material|SetMaterial _cube 0 _output_get))

(event EventInteract
  (if (Variables|Default|GetScucced)
    (Development|PrintString "interacting" true true "(R=0.000000,G=0.660000,B=1.000000,A=1.000000)" 3.0)
    (Variables|Default|SetScucced false)
    (bind _outactors (Actor|GetAllActorsOfClass "/Game/FirstPerson/Blueprints/BP_FirstPersonCharacter.BP_FirstPersonCharacter_C"))
    (Default|ColorIncriment (Utilities|Array|Get(acopy) _outactors) (Variables|Default|GetColorIndex))
    (bind _asactor (Utilities|Casting|CastToActor (.HitActor (Collision|BreakHitResult (.HitResult (Class|PlayerController|GetHitResultUnderCursorforObjects (Game|GetPlayerController 0) (Utilities|Array|MakeArray "ObjectTypeQuery2") true))))))
    (CallFunction|ThisTime 0.5 (Math|Vector2D|MakeVector2D (Math|Float|MapRangeClamped (.x (Math|Vector|Normalize (+ (Math|Transform|InverseTransformDirection (Transformation|GetWorldTransform (Variables|/Script/Engine.Actor|GetRootComponent _asactor)) "0, 0, 0") (Math|Vector|MakeVector 0.0 0.0 (* (.z (.BoxExtent (Collision|GetComponentBounds (Variables|/Script/Engine.Actor|GetRootComponent _asactor)))) 0.5))))) 0.0 0.0 0.0 0.0) (Math|Float|MapRangeClamped (.y (Math|Vector|Normalize (+ (Math|Transform|InverseTransformDirection (Transformation|GetWorldTransform (Variables|/Script/Engine.Actor|GetRootComponent _asactor)) "0, 0, 0") (Math|Vector|MakeVector 0.0 0.0 (* (.z (.BoxExtent (Collision|GetComponentBounds (Variables|/Script/Engine.Actor|GetRootComponent _asactor)))) 0.5))))) 0.0 0.0 0.0 0.0)))))

(event Input|MouseEvents|LeftMouseButton
  (params (Key :type Key%20Structure :default "None")))

(fn ConstructionScript)